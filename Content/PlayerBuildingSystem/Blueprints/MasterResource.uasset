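; Base harvestable resource actor for the player building system, holding wood and stone amounts.
; On Interact it harvests a fixed amount and reports it to the PlayerBuildingComponent via ServerResourceCollected.
; ResourceCollected draws wood before stone and destroys the actor when that resource empties or both are empty.
; A remainder smaller than the harvest still yields the full amount without deduction; the destroy calls for that case are unwired.
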(event `/Game/PlayerBuildingSystem/Blueprints/BuildingBlueprints/Other/BuildingInterface.Interact`
  (params (`Player Building Component` :type "/Game/PlayerBuildingSystem/Blueprints/Components/PlayerBuildingComponent Object Reference"))
  (bind _resouses (`self.Resource Collected` 10))
  (`/Game/PlayerBuildingSystem/Blueprints/Components/PlayerBuildingComponent.Server Resource Collected` `Player Building Component` _resouses))

(fn `Resource Collected`
  (params (`Collected Amount` :type Integer))
  (returns (Resouses :type "/Game/PlayerBuildingSystem/Blueprints/BuildingBlueprints/Other/S_BuildingCost Structure"))
  (locals (`Harvested Amount L` :type Integer))
  (set `local.Harvested Amount L` `Collected Amount`)
  (if (> (break `/Game/PlayerBuildingSystem/Blueprints/BuildingBlueprints/Other/S_ResourceCost` (break `/Game/PlayerBuildingSystem/Blueprints/BuildingBlueprints/Other/S_BuildingCost` (`self.Resources`))) 0)
    (if (>= (break `/Game/PlayerBuildingSystem/Blueprints/BuildingBlueprints/Other/S_ResourceCost` (break `/Game/PlayerBuildingSystem/Blueprints/BuildingBlueprints/Other/S_BuildingCost` (`self.Resources`))) (`local.Harvested Amount L`))
      (bind _output_get (set `self.Resources` (make `/Game/PlayerBuildingSystem/Blueprints/BuildingBlueprints/Other/S_BuildingCost` (make `/Game/PlayerBuildingSystem/Blueprints/BuildingBlueprints/Other/S_ResourceCost` (- (break `/Game/PlayerBuildingSystem/Blueprints/BuildingBlueprints/Other/S_ResourceCost` (break `/Game/PlayerBuildingSystem/Blueprints/BuildingBlueprints/Other/S_BuildingCost` (`self.Resources`))) (`local.Harvested Amount L`))))))
      (if (not (> (break `/Game/PlayerBuildingSystem/Blueprints/BuildingBlueprints/Other/S_ResourceCost` (break `/Game/PlayerBuildingSystem/Blueprints/BuildingBlueprints/Other/S_BuildingCost` _output_get)) 0))
        (`self.K2_DestroyActor`))
      (return (make `/Game/PlayerBuildingSystem/Blueprints/BuildingBlueprints/Other/S_BuildingCost` (make `/Game/PlayerBuildingSystem/Blueprints/BuildingBlueprints/Other/S_ResourceCost` (`local.Harvested Amount L`))))
      (else
        (return (make `/Game/PlayerBuildingSystem/Blueprints/BuildingBlueprints/Other/S_BuildingCost` (make `/Game/PlayerBuildingSystem/Blueprints/BuildingBlueprints/Other/S_ResourceCost` (`local.Harvested Amount L`))))))
    (elif (> (break `/Game/PlayerBuildingSystem/Blueprints/BuildingBlueprints/Other/S_ResourceCost` (`.Stone_8_845E236D46B31C45609676924CCE7CB0` (break `/Game/PlayerBuildingSystem/Blueprints/BuildingBlueprints/Other/S_BuildingCost` (`self.Resources`)))) 0)
      (if (>= (break `/Game/PlayerBuildingSystem/Blueprints/BuildingBlueprints/Other/S_ResourceCost` (`.Stone_8_845E236D46B31C45609676924CCE7CB0` (break `/Game/PlayerBuildingSystem/Blueprints/BuildingBlueprints/Other/S_BuildingCost` (`self.Resources`)))) (`local.Harvested Amount L`))
        (bind _output_get_2 (set `self.Resources` (make `/Game/PlayerBuildingSystem/Blueprints/BuildingBlueprints/Other/S_BuildingCost` (struct) (make `/Game/PlayerBuildingSystem/Blueprints/BuildingBlueprints/Other/S_ResourceCost` (- (break `/Game/PlayerBuildingSystem/Blueprints/BuildingBlueprints/Other/S_ResourceCost` (`.Stone_8_845E236D46B31C45609676924CCE7CB0` (break `/Game/PlayerBuildingSystem/Blueprints/BuildingBlueprints/Other/S_BuildingCost` (`self.Resources`)))) (`local.Harvested Amount L`))))))
        (if (not (> (break `/Game/PlayerBuildingSystem/Blueprints/BuildingBlueprints/Other/S_ResourceCost` (`.Stone_8_845E236D46B31C45609676924CCE7CB0` (break `/Game/PlayerBuildingSystem/Blueprints/BuildingBlueprints/Other/S_BuildingCost` _output_get_2))) 0))
          (`self.K2_DestroyActor`))
        (return (make `/Game/PlayerBuildingSystem/Blueprints/BuildingBlueprints/Other/S_BuildingCost` (struct) (make `/Game/PlayerBuildingSystem/Blueprints/BuildingBlueprints/Other/S_ResourceCost` (`local.Harvested Amount L`))))
        (else
          (return (make `/Game/PlayerBuildingSystem/Blueprints/BuildingBlueprints/Other/S_BuildingCost` (struct) (make `/Game/PlayerBuildingSystem/Blueprints/BuildingBlueprints/Other/S_ResourceCost` (`local.Harvested Amount L`))))))
      (else
        (`self.K2_DestroyActor`)
        (return)))))

(fn `UserConstructionScript`)